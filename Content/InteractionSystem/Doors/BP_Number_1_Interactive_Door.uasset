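; BP_Number_1_Interactive_Door is one digit of an interactive door's code, shown on a TextRender.
; Two events step the digit up or down, wrapping between 1 and 9.
; Each change flags whether it equals the hardcoded answer 4 on BP_Number_0_Interactive_Door, calls its CheckCode, then updates the text.
; That reference is found at BeginPlay via GetAllActorsOfClass, keeping the last instance found.
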(event Custom|+1%20Set%20Number%201
  ;[0 0 0] Système de modification du numéro de la porte associé
  (if (< (Variables|Default|GetVariable%20Gestion%20Numero%201%20Affiche) 9.0)
    (Variables|Default|SetVariable%20Gestion%20Numero%201%20Affiche (+ (Variables|Default|GetVariable%20Gestion%20Numero%201%20Affiche) 1.0))
    (else
      (Variables|Default|SetVariable%20Gestion%20Numero%201%20Affiche 1.0)))
  ;[0 0 0] Vérification du code et système d'ouverture de la porte
  (if (== (Variables|Default|GetVariable%20Gestion%20Numero%201%20Affiche) 4.0)
    (bind _asbp_number_0_interactive_door (Utilities|Casting|CastToBP_Number_0_Interactive_Door (Variables|Default|GetRef%20Number%200)))
    (Variables|/Game/InteractionSystem/Doors/BP_Number_0_Interactive_Door.BP_Number_0_Interactive_Door_C|SetIsNumber1Correct? _asbp_number_0_interactive_door true)
    (else
      (bind _asbp_number_0_interactive_door_2 (Utilities|Casting|CastToBP_Number_0_Interactive_Door (Variables|Default|GetRef%20Number%200)))
      (Variables|/Game/InteractionSystem/Doors/BP_Number_0_Interactive_Door.BP_Number_0_Interactive_Door_C|SetIsNumber1Correct? _asbp_number_0_interactive_door_2 false)))
  (bind _asbp_number_0_interactive_door_3 (Utilities|Casting|CastToBP_Number_0_Interactive_Door (Variables|Default|GetRef%20Number%200)))
  (Default|CheckCode _asbp_number_0_interactive_door_3)
  (Rendering|Components|TextRender|SetText (Variables|Default|GetTextRender) (Utilities|Text|ToText(Float) (Variables|Default|GetVariable%20Gestion%20Numero%201%20Affiche) "HalfToEven")))

(event Custom|-1%20Set%20Number%201
  ;[0 0 0] Système de modification du numéro de la porte associé
  (if (> (Variables|Default|GetVariable%20Gestion%20Numero%201%20Affiche) 1.0)
    (Variables|Default|SetVariable%20Gestion%20Numero%201%20Affiche (- (Variables|Default|GetVariable%20Gestion%20Numero%201%20Affiche) 1.0))
    (else
      (Variables|Default|SetVariable%20Gestion%20Numero%201%20Affiche 9.0)))
  ;[0 0 0] Vérification du code et système d'ouverture de la porte
  (if (== (Variables|Default|GetVariable%20Gestion%20Numero%201%20Affiche) 4.0)
    (bind _asbp_number_0_interactive_door (Utilities|Casting|CastToBP_Number_0_Interactive_Door (Variables|Default|GetRef%20Number%200)))
    (Variables|/Game/InteractionSystem/Doors/BP_Number_0_Interactive_Door.BP_Number_0_Interactive_Door_C|SetIsNumber1Correct? _asbp_number_0_interactive_door true)
    (else
      (bind _asbp_number_0_interactive_door_2 (Utilities|Casting|CastToBP_Number_0_Interactive_Door (Variables|Default|GetRef%20Number%200)))
      (Variables|/Game/InteractionSystem/Doors/BP_Number_0_Interactive_Door.BP_Number_0_Interactive_Door_C|SetIsNumber1Correct? _asbp_number_0_interactive_door_2 false)))
  (bind _asbp_number_0_interactive_door_3 (Utilities|Casting|CastToBP_Number_0_Interactive_Door (Variables|Default|GetRef%20Number%200)))
  (Default|CheckCode _asbp_number_0_interactive_door_3)
  (Rendering|Components|TextRender|SetText (Variables|Default|GetTextRender) (Utilities|Text|ToText(Float) (Variables|Default|GetVariable%20Gestion%20Numero%201%20Affiche) "HalfToEven")))

(event EventBeginPlay
  (bind _outactors (Actor|GetAllActorsOfClass "/Game/InteractionSystem/Doors/BP_Number_0_Interactive_Door.BP_Number_0_Interactive_Door_C"))
  (for _array_element _outactors
    (Variables|Default|SetRef%20Number%200 _array_element)))

(fn ConstructionScript)