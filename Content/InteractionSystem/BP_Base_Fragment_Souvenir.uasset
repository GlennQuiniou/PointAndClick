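; Base Blueprint for a "Fragment Souvenir" interactable sphere that toggles color and size, intended to follow the character's size.
; Fragment_Souvenir_Change_Size flips IsWhite and plays a white/blue color timeline on a dynamic material created in the Construction Script.
; When the color finishes, a shared timeline lerps the sphere between its initial scale and a version doubled in X and Y.
; Interact_Fragment_Souvenir only prints a debug message.
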(event Custom|Fragment_Souvenir_Change_Size
  ;[0 0 0] Change la taille et la couleur du Fragment Souvenir en fonction de la taille du personnnage
  (if (Variables|Default|GetIsWhite?)
    (Variables|Default|SetIsWhite? false)
    (bind _track_color (Timeline|Timeline_Color_White_To_Blue PlayFromStart)
      (:Update
        (Rendering|Material|SetVectorParameterValue (Variables|Default|GetVariableDynamicMaterialInstance) "Color" _track_color :!class /Script/Engine.MaterialInstanceDynamic))
      (:Finished
        (Variables|Default|SetNewSize (Variables|Default|GetSizeBlue))
        (bind _track_size (Timeline|Timeline_Size_Fragment_Souvenir PlayFromStart)
          (:Update
            (Transformation|SetWorldScale3D (Variables|Default|GetSphere) (Math|Vector|Lerp(Vector) (Transformation|GetWorldScale (Variables|Default|GetSphere)) (Variables|Default|GetNewSize) _track_size))))))
    (else
      (Variables|Default|SetIsWhite? true)
      (bind _track_color_2 (Timeline|Timeline_Color_Blue_To_White PlayFromStart)
        (:Update
          (Rendering|Material|SetVectorParameterValue (Variables|Default|GetVariableDynamicMaterialInstance) "Color" _track_color_2 :!class /Script/Engine.MaterialInstanceDynamic))
        (:Finished
          (Variables|Default|SetNewSize (Variables|Default|GetDefaultSize))
          (Timeline|Timeline_Size_Fragment_Souvenir PlayFromStart))))))

(event Custom|Interact_Fragment_Souvenir
  (Development|PrintString "Interact Fragment Souvenir Fonctionne"))

(event EventBeginPlay
  (bind _sphere (Variables|Default|GetSphere))
  (bind _returnvalue (Transformation|GetWorldScale _sphere))
  ;[0 0 0] Définit les variables de défaut
  (Variables|Default|SetIsWhite? true)
  (Variables|Default|SetDefaultSize (Transformation|GetWorldScale (Variables|Default|GetSphere)))
  (Variables|Default|SetSizeBlue (Math|Vector|MakeVector (* (.x _returnvalue) 2.0) (* (.y _returnvalue) 2.0) (.z _returnvalue))))

(fn ConstructionScript
  (bind _returnvalue (Rendering|Material|CreateDynamicMaterialInstance (Variables|Default|GetSphere) 0 0 "None" :!class /Script/Engine.PrimitiveComponent))
  (Variables|Default|SetVariableDynamicMaterialInstance _returnvalue))