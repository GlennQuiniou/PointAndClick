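; BP_InteractActor_Test_2 is a test interactable TV that toggles on and off, built on a parent class's Interact event.
; It sets IsOn true at BeginPlay, then each interaction flips it, pausing or resuming the Sea of Love audio.
; Each toggle also creates a dynamic material instance from the on or off TV material on the mesh.
; The audio's Play call is disconnected and never runs.
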(event EventBeginPlay
  (|CallParentFunction)
  ;[0 0 0] Pour la faire fonctionner à nouveau il faut relier ces blueprint là
  (Variables|Default|SetisOn? true))

(event Collision|EventActorBeginOverlap
  (params (OtherActor :type Actor%20Object%20Reference)))

(event EventTick
  (params (DeltaSeconds :type Float%20%28single-precision%29)))

(event EventInteract
  (|CallParentFunction)
  (bind _output_get (Variables|Default|SetisOn? (not (Variables|Default|GetisOn?))))
  (if _output_get
    (Class|AudioComponent|SetPaused (Variables|Default|GetAudio%20-%20SeaOfLove) false)
    (Rendering|Material|CreateDynamicMaterialInstance (Variables|Default|GetStaticMesh) 0 "/Game/DetectiveStart/Assets/Materials/M_TV.M_TV" "None" :!class /Script/Engine.PrimitiveComponent)
    (else
      (Class|AudioComponent|SetPaused (Variables|Default|GetAudio%20-%20SeaOfLove) true)
      (Rendering|Material|CreateDynamicMaterialInstance (Variables|Default|GetStaticMesh) 0 "/Game/DetectiveStart/Assets/Materials/M_TV_Off.M_TV_Off" "None" :!class /Script/Engine.PrimitiveComponent))))

(fn ConstructionScript
  (|CallParentFunction))